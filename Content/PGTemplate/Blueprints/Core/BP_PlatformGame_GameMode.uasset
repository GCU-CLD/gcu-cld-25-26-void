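; Platformer game mode that runs a level's flow from intro and camera fade to end screen, pause menu and next-level travel.
; BeginPlay counts collectibles, builds the HUD, caches switches, maps patrol nodes by route and node ID, and prints level-setup warnings.
; Collectible events update the HUD; collecting all mandatory ones opens the level end.
; Pause and completion swap Enhanced Input contexts; the next level comes from a data table, falling back to Menu.
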(event `self.ReceiveBeginPlay`
  (bind _returnvalue (`GameplayStatics.GetPlayerController` 0))
  (bind _patrolnodes (`self.PatrolNodes`))
  ;[1 1 1] BeginPlay Actions
  (`WidgetBlueprintLibrary.SetInputMode_GameOnly` _returnvalue)
  (set `PlayerController.bShowMouseCursor` false _returnvalue)
  (`/Game/PGTemplate/Blueprints/Characters/Player/BP_PlatformGameCameraManager.FadeIn` (cast `/Game/PGTemplate/Blueprints/Characters/Player/BP_PlatformGameCameraManager` (`GameplayStatics.GetPlayerCameraManager` 0) :!pure true) 2.0)
  (`|ExecutionSequence`
    (:`then_0`
      (bind _outactors (`GameplayStatics.GetAllActorsOfClass` "/Game/PGTemplate/Blueprints/Objects/Collectibles/OptionalCollectible_BP.OptionalCollectible_BP_C"))
      (set `self.OptionalCollectiblesInLevel` (`KismetArrayLibrary.Array_Length` _outactors)))
    (:`then_1`
      (bind _outactors_2 (`GameplayStatics.GetAllActorsOfClass` "/Game/PGTemplate/Blueprints/Objects/Collectibles/MandatoryCollectible_BP.MandatoryCollectible_BP_C"))
      (set `self.MandatoryCollectiblesInLevel` (`KismetArrayLibrary.Array_Length` _outactors_2))
      (bind _outactors_3 (`GameplayStatics.GetAllActorsOfClass` "/Game/PGTemplate/Blueprints/Objects/LevelEnd_BP.LevelEnd_BP_C"))
      (`/Engine/EditorBlueprintResources/StandardMacros.CompareInt` (`KismetArrayLibrary.Array_Length` _outactors_3) 1
        (:`>`
          (`KismetSystemLibrary.PrintString` "MULTIPLE LEVEL ENDS DETECTED"))
        (:`==`
          (bind _output_get (set `self.LevelEnd` (`|GetArrayItem` _outactors_3)))
          (if (== (`self.MandatoryCollectiblesInLevel`) 0)
            (`/Game/PGTemplate/Blueprints/Objects/LevelEnd_BP.Open` _output_get)))
        (:`<`
          (`KismetSystemLibrary.PrintString` "NO LEVEL END DETECTED"))))
    (:`then_2`
      ;;[0 0 0] Set up HUD Widget
      (bind _returnvalue_2 (`|CreateWidget` "/Game/PGTemplate/Blueprints/Characters/Player/UI/PlayerHUD_W.PlayerHUD_W_C"))
      (bind _output_get_2 (set `self.PlayerHUD` _returnvalue_2))
      (`UserWidget.AddToViewport` _output_get_2 0)
      (`/Game/PGTemplate/Blueprints/Characters/Player/UI/PlayerHUD_W.UpdateCollectiblesCount` (`self.PlayerHUD`) 0 (`self.MandatoryCollectiblesInLevel`) 0 (`self.OptionalCollectiblesInLevel`)))
    (:`then_3`
      ;;[1 0 0] PRINT WARNING ERROR IF ENEMIES EXIST BUT NAV MESH DOES NOT
      (bind _outactors_4 (`GameplayStatics.GetAllActorsOfClass` "/Game/PGTemplate/Blueprints/Characters/Enemy/Core/BP_Enemy_Base.BP_Enemy_Base_C"))
      (if (> (`KismetArrayLibrary.Array_Length` _outactors_4) 0)
        (bind _outactors_5 (`GameplayStatics.GetAllActorsOfClass` "/Script/NavigationSystem.NavMeshBoundsVolume"))
        (if (not (> (`KismetArrayLibrary.Array_Length` _outactors_5) 0))
          (`KismetSystemLibrary.PrintString` "!!!!!!!! WARNING: ENEMIES PLACED IN MAP BUT NO NAVMESH IS PRESENT IN LEVEL \n(Read this line to Alan if asking for help with this problem)" true true (struct :`R` 1.0 :`A` 1.0) 10.0))))
    (:`then_4`
      ;;[0 0 0] Organise Patrol Nodes into 3D Map
      (bind _outactors_6 (`GameplayStatics.GetAllActorsOfClass` "/Game/PGTemplate/Blueprints/Objects/LogicTriggers/EnemyPatrolNode_BP.EnemyPatrolNode_BP_C"))
      (for _array_element _outactors_6
        (bind _returnvalue_3 (`KismetMathLibrary.Conv_IntToDouble` (`/Game/PGTemplate/Blueprints/Objects/LogicTriggers/EnemyPatrolNode_BP.RouteID` _array_element)))
        (bind _returnvalue_4 (`KismetMathLibrary.Conv_IntToDouble` (`/Game/PGTemplate/Blueprints/Objects/LogicTriggers/EnemyPatrolNode_BP.NodeID` _array_element)))
        (bind (_value _returnvalue_5) (`BlueprintMapLibrary.Map_Find` _patrolnodes (`KismetMathLibrary.MakeVector2D` _returnvalue_3 _returnvalue_4)))
        (if _returnvalue_5
          (`KismetSystemLibrary.PrintString` (`KismetStringLibrary.Concat_StrStr` "Patrol Node " (`KismetSystemLibrary.GetDisplayName` _value) " has the same Route & Node ID as Patrol Node " (`KismetSystemLibrary.GetDisplayName` _array_element)))
          (else
            (`BlueprintMapLibrary.Map_Add` _patrolnodes (`KismetMathLibrary.MakeVector2D` _returnvalue_3 _returnvalue_4) _array_element)))))
    (:`then_5`
      (bind _outactors_7 (`GameplayStatics.GetAllActorsOfClass` "/Game/PGTemplate/Blueprints/Objects/Switches/IO_Switch_BP.IO_Switch_BP_C"))
      (set `self.AllSwitchesInLevel` _outactors_7))
    (:`then_6`
      ;;[1 1 1] Add Level Intro
      (bind _returnvalue_6 (`|CreateWidget` "/Game/PGTemplate/UI/LevelIntro_UI.LevelIntro_UI_C"))
      (`UserWidget.AddToViewport` _returnvalue_6 0))))

(event `LevelComplete`
  (bind _returnvalue (pcsubsystem `EnhancedInputLocalPlayerSubsystem` (`GameplayStatics.GetPlayerController` 0)))
  ;[1 1 1] LevelComplete
  (set `/Game/PGTemplate/Blueprints/Characters/Player/BP_PlatformGameCameraManager.TrackedActor` (`self.LevelEnd`) (cast `/Game/PGTemplate/Blueprints/Characters/Player/BP_PlatformGameCameraManager` (`GameplayStatics.GetPlayerCameraManager` 0) :!pure true))
  (bind _returnvalue_2 (`|CreateWidget` "/Game/PGTemplate/Blueprints/Core/LevelEndScreen_W.LevelEndScreen_W_C"))
  (bind _output_get (set `self.LevelEndWidget` _returnvalue_2))
  (`UserWidget.AddToViewport` _output_get 0)
  (`EnhancedInputSubsystemInterface.ClearAllMappings` _returnvalue)
  (`EnhancedInputSubsystemInterface.AddMappingContext` _returnvalue "/Game/PGTemplate/Blueprints/Characters/Player/Input/IMC_EndScreen.IMC_EndScreen" 0 (struct)))

(event `NextLevel`
  ;[1 1 1] LevelComplete
  (`/Game/PGTemplate/Blueprints/Characters/Player/BP_PlatformGameCameraManager.FadeOut` (cast `/Game/PGTemplate/Blueprints/Characters/Player/BP_PlatformGameCameraManager` (`GameplayStatics.GetPlayerCameraManager` 0) :!pure true) 1.0)
  (`KismetSystemLibrary.Delay` 1.0)
  (bind _returnvalue (`GameplayStatics.GetCurrentLevelName` true))
  (bind _returnvalue_2 (`|GetDataTableRow` "/Game/PGTemplate/Maps/LevelData_DT.LevelData_DT" (`KismetStringLibrary.Conv_StringToName` _returnvalue))
    (:`then`
      (`GameplayStatics.OpenLevel` (`KismetStringLibrary.Conv_StringToName` (`.NextLevelName_9_524B3ADE4136531C2984D8AC2B73D776` (break `/Game/PGTemplate/Maps/LevelDataRow` _returnvalue_2)))))
    (:`RowNotFound`
      (`GameplayStatics.OpenLevel` "Menu"))))

(event `PauseGame`
  (bind _returnvalue (pcsubsystem `EnhancedInputLocalPlayerSubsystem` (`GameplayStatics.GetPlayerController` 0)))
  ;[1 1 1] Pause & Unpasue Game
  (`GameplayStatics.SetGamePaused` true)
  (bind _returnvalue_2 (`|CreateWidget` "/Game/PGTemplate/UI/PauseMenu_W.PauseMenu_W_C"))
  (bind _output_get (set `self.PauseMenu` _returnvalue_2))
  (`UserWidget.AddToViewport` _output_get 0)
  (`EnhancedInputSubsystemInterface.ClearAllMappings` _returnvalue)
  (`EnhancedInputSubsystemInterface.AddMappingContext` _returnvalue "/Game/PGTemplate/Blueprints/Characters/Player/Input/IMC_Dialog.IMC_Dialog" 0 (struct)))

(event `UnPauseGame`
  (bind _returnvalue (`GameplayStatics.GetPlayerController` 0))
  (bind _returnvalue_2 (pcsubsystem `EnhancedInputLocalPlayerSubsystem` (`GameplayStatics.GetPlayerController` 0)))
  ;[1 1 1] Pause & Unpasue Game
  (`WidgetBlueprintLibrary.SetInputMode_GameOnly` _returnvalue)
  (set `PlayerController.bShowMouseCursor` false _returnvalue)
  (`GameplayStatics.SetGamePaused` false)
  (`Widget.RemoveFromParent` (`self.PauseMenu`))
  (`EnhancedInputSubsystemInterface.ClearAllMappings` _returnvalue_2)
  (`EnhancedInputSubsystemInterface.AddMappingContext` _returnvalue_2 "/Game/PGTemplate/Blueprints/Characters/Player/Input/IMC_Default.IMC_Default" 0 (struct)))

(event `MandatoryCollectibleCollected`
  (bind _result (`/Engine/EditorBlueprintResources/StandardMacros.IncrementInt` (`self.MandatoryCollectiblesCollected`))
    (:`  `
      (if (== _result (`self.MandatoryCollectiblesInLevel`))
        (`/Game/PGTemplate/Blueprints/Objects/LevelEnd_BP.Open` (`self.LevelEnd`)))
      (`/Game/PGTemplate/Blueprints/Characters/Player/UI/PlayerHUD_W.UpdateCollectiblesCount` (`self.PlayerHUD`) (`self.MandatoryCollectiblesCollected`) (`self.MandatoryCollectiblesInLevel`) (`self.OptionalCollectiblesCollected`) (`self.OptionalCollectiblesInLevel`) :!label _label))))

(event `OptionalCollectibleCollected`
  (`/Engine/EditorBlueprintResources/StandardMacros.IncrementInt` (`self.OptionalCollectiblesCollected`)
    (:`  `
      (goto _label))))

(fn `UserConstructionScript`)